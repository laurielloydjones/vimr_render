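; Player controller for the VR Powhiri experience that turns right Oculus trigger presses into either voxel video selection or teleporting.
; BeginPlay caches the pawn and voxel video player, and maps "marker" actors by tag.
; A short ray from the motion controller resolves a hit's parent tag to a marker transform for SelectVoxelVideo.
; Misses show the teleport, executed on release; Escape quits.
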(event `self.ReceiveBeginPlay`
  (`self.SetControlledPawn`)
  (`self.FindVoxelVideoPlayer`)
  (`self.GetAllMarkers`))

(event `InputAction|OculusRightTrigger`
  (params (Key :type "Key Structure"))
  (bind _powhiripawnref (`self.PowhiriPawnRef`))
  (:`Pressed`
    (bind (_returnvalue _tagname) (`self.CastSelectionRay2` _powhiripawnref)
      (:`OnSelectable`
        (`/Game/Blueprints/Actors/VoxelVideoActor.SelectVoxelVideo` (`self.VoxelVideoPlayer`) _tagname _returnvalue))
      (:`NotSelectable`
        (`/Game/Blueprints/Pawns/PowhiriPawn.ShowTeleport` _powhiripawnref "Right"))))
  (:`Released`
    (if (not (`self.OnSelectable`))
      (`/Game/Blueprints/Pawns/PowhiriPawn.ExecTeleport` _powhiripawnref "Right"))
    (set `self.OnSelectable` false)))

(event `Key|Escape`
  (params (Key :type "Key Structure"))
  ;[1 1 1] Exit Game
  (:`Pressed`
    (`KismetSystemLibrary.QuitGame` null "Quit")))

(fn `CastSelectionRay`
  (params (PowhiriPawn :type "/Game/Blueprints/Pawns/PowhiriPawn Object Reference"))
  (returns (TagName :type Name) (MarkerTransform :type "Transform Structure"))
  (bind _right (`/Game/Blueprints/Pawns/PowhiriPawn.Right` PowhiriPawn))
  (bind _returnvalue (`SceneComponent.K2_GetComponentLocation` _right))
  (if (`/Game/Blueprints/Pawns/PowhiriPawn.IsUsingHmd` PowhiriPawn)
    (bind (_outhit _returnvalue_2) (`KismetSystemLibrary.LineTraceSingle` :`Start` _returnvalue :`End` (+ _returnvalue (* (`KismetMathLibrary.GetForwardVector` (`SceneComponent.K2_GetComponentRotation` _right)) 200.0)) :`TraceChannel` "TraceTypeQuery3" :`TraceColor` (struct :`R` 0.17387 :`G` 0.880208 :`A` 1.0) :`DrawTime` 10.0))
    (if _returnvalue_2
      (bind _output (`|GetArrayItem` (`Actor.Tags` (`self.GetAttachParentActor` (`.HitActor` (`GameplayStatics.BreakHitResult` _outhit))))))
      (return _output (`self.GetTransform` (`BlueprintMapLibrary.Map_Find` (`self.MarkerActors`) _output))))))

(fn `FindVoxelVideoPlayer`
  (bind _outactors (`GameplayStatics.GetAllActorsOfClass` "/Game/Blueprints/Actors/VoxelVideoActor.VoxelVideoActor_C"))
  (set `self.VoxelVideoPlayer` (`|GetArrayItem` _outactors)))

(fn `GetAllMarkers`
  (bind _outactors (`GameplayStatics.GetAllActorsWithTag` "marker"))
  (for _array_element _outactors
    (`BlueprintMapLibrary.Map_Add` (`self.MarkerActors`) (`|GetArrayItem` (`Actor.Tags` _array_element)) _array_element)))

(fn `SetControlledPawn`
  (bind _aspowhiri_pawn (cast `/Game/Blueprints/Pawns/PowhiriPawn` (`self.K2_GetPawn`))
    (:`then`
      (set `self.PowhiriPawnRef` _aspowhiri_pawn))
    (:`CastFailed`
      (`KismetSystemLibrary.PrintString` "Failed to Cast to VrPawn!" false true (struct :`G` 0.66 :`B` 1.0 :`A` 1.0) 10.0))))

(fn `UserConstructionScript`)