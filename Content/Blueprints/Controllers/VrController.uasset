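; VR player controller that forwards Oculus trigger input to the possessed VrPawn for teleporting and quits the game on Escape.
; Each trigger shows that hand's teleport on press and executes it on release, relying on a navmesh volume.
; BeginPlay caches the pawn and first VoxelVideoActor, and fills a marker map keyed by first tag, though its actor search uses the "None" tag.
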(event `self.ReceiveBeginPlay`
  (`self.SetControlledPawn`)
  (`self.FindVoxelVideoPlayer`)
  (`self.GetAllMarkers`))

(event `InputAction|OculusRightTrigger`
  (params (Key :type "Key Structure"))
  (bind _vrpawnref (`self.VrPawnRef`))
  ;[1 1 1] Teleport - this requires a navmesh volume in the world
  (:`Pressed`
    (`/Game/Blueprints/Pawns/VrPawn.ShowTeleport` _vrpawnref "Right"))
  (:`Released`
    (`/Game/Blueprints/Pawns/VrPawn.ExecTeleport` _vrpawnref "Right")))

(event `InputAction|OculusLeftTrigger`
  (params (Key :type "Key Structure"))
  (bind _vrpawnref (`self.VrPawnRef`))
  ;[1 1 1] Teleport - this requires a navmesh volume in the world
  (:`Pressed`
    (`/Game/Blueprints/Pawns/VrPawn.ShowTeleport` _vrpawnref "Left"))
  (:`Released`
    (`/Game/Blueprints/Pawns/VrPawn.ExecTeleport` _vrpawnref "Left")))

(event `Key|Escape`
  (params (Key :type "Key Structure"))
  ;[1 1 1] Exit Game
  (:`Pressed`
    (`KismetSystemLibrary.QuitGame` null "Quit")))

(fn `FindVoxelVideoPlayer`
  (bind _outactors (`GameplayStatics.GetAllActorsOfClass` "/Game/Blueprints/Actors/VoxelVideoActor.VoxelVideoActor_C"))
  (set `self.VoxelVideoPlayer` (`|GetArrayItem` _outactors)))

(fn `GetAllMarkers`
  (bind _outactors (`GameplayStatics.GetAllActorsWithTag` "None"))
  (for _array_element _outactors
    (`BlueprintMapLibrary.Map_Add` (`self.MarkerActors`) (`|GetArrayItem` (`Actor.Tags` _array_element)) _array_element)))

(fn `SetControlledPawn`
  (bind _asvr_pawn (cast `/Game/Blueprints/Pawns/VrPawn` (`self.K2_GetPawn`))
    (:`then`
      (set `self.VrPawnRef` _asvr_pawn))
    (:`CastFailed`
      (`KismetSystemLibrary.PrintString` "Failed to Cast to VrPawn!" false true (struct :`G` 0.66 :`B` 1.0 :`A` 1.0) 10.0))))

(fn `UserConstructionScript`)