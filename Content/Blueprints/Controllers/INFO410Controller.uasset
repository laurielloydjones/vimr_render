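; Player controller for a VR scene that lets Oculus triggers either toggle voxel video playback or teleport the VR pawn.
; On BeginPlay it caches the controlled VrPawn and the first VoxelVideoActor found in the level.
; Each trigger press line-traces from that hand: hitting a "Button"-tagged actor toggles playback, otherwise it shows the navmesh-dependent teleport, executed on release.
; Escape quits the game.
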(event `self.ReceiveBeginPlay`
  (`self.SetControlledPawn`)
  (`self.GetVoxelVideoReference`))

(event `InputAction|OculusRightTrigger`
  (params (Key :type "Key Structure"))
  (bind _vrpawnref (`self.VrPawnRef`))
  ;[1 1 1] Teleport - this requires a navmesh volume in the world
  (:`Pressed`
    (bind _isbuttonhit_ (`self.CastVoxelVideoPlay` (`/Game/Blueprints/Pawns/VrPawn.RightController` (`self.VrPawnRef`))))
    (if _isbuttonhit_
      (set `self.IsButtonSelected` true)
      (else
        (`/Game/Blueprints/Pawns/VrPawn.ShowTeleport` _vrpawnref "Right"))))
  (:`Released`
    (if (`self.IsButtonSelected`)
      (set `self.IsButtonSelected` false)
      (else
        (`/Game/Blueprints/Pawns/VrPawn.ExecTeleport` _vrpawnref "Right")))))

(event `InputAction|OculusLeftTrigger`
  (params (Key :type "Key Structure"))
  (bind _vrpawnref (`self.VrPawnRef`))
  ;[1 1 1] Teleport - this requires a navmesh volume in the world
  (:`Pressed`
    (bind _isbuttonhit_ (`self.CastVoxelVideoPlay` (`/Game/Blueprints/Pawns/VrPawn.LeftController` (`self.VrPawnRef`))))
    (if _isbuttonhit_
      (set `self.IsButtonSelected` true)
      (else
        (`/Game/Blueprints/Pawns/VrPawn.ShowTeleport` _vrpawnref "Left"))))
  (:`Released`
    (if (`self.IsButtonSelected`)
      (set `self.IsButtonSelected` false)
      (else
        (`/Game/Blueprints/Pawns/VrPawn.ExecTeleport` _vrpawnref "Left")))))

(event `Key|Escape`
  (params (Key :type "Key Structure"))
  ;[1 1 1] Exit Game
  (:`Pressed`
    (`KismetSystemLibrary.QuitGame` null "Quit")))

(fn `CastVoxelVideoPlay`
  (params (VrHandActor :type "/Game/Blueprints/Actors/VrHandActor Object Reference"))
  (returns (`IsButtonHit?` :type Boolean))
  (bind _motioncontroller (`/Game/Blueprints/Actors/VrHandActor.MotionController` VrHandActor))
  (bind _returnvalue (`SceneComponent.K2_GetComponentLocation` _motioncontroller))
  (bind (_outhit _returnvalue_2) (`KismetSystemLibrary.LineTraceSingle` _returnvalue (+ _returnvalue (* (`SceneComponent.GetForwardVector` _motioncontroller) 5000)) "TraceTypeQuery1"))
  (if _returnvalue_2
    (bind _returnvalue_3 (`self.ActorHasTag` (`.HitActor` (`GameplayStatics.BreakHitResult` _outhit)) "Button"))
    (if _returnvalue_3
      (`/Game/Blueprints/Actors/VoxelVideoActor.TogglePlay` (`self.VoxelVideoRef`))
      (return _returnvalue_3)
      (else
        (return _returnvalue_3)))
    (else
      (return _returnvalue_2))))

(fn `GetVoxelVideoReference`
  (bind _outactors (`GameplayStatics.GetAllActorsOfClass` "/Game/Blueprints/Actors/VoxelVideoActor.VoxelVideoActor_C"))
  (set `self.VoxelVideoRef` (`|GetArrayItem` _outactors)))

(fn `SetControlledPawn`
  (bind _asvr_pawn (cast `/Game/Blueprints/Pawns/VrPawn` (`self.K2_GetPawn`))
    (:`then`
      (set `self.VrPawnRef` _asvr_pawn))
    (:`CastFailed`
      (`KismetSystemLibrary.PrintString` "Failed to Cast to VrPawn!" false true (struct :`G` 0.66 :`B` 1.0 :`A` 1.0) 10.0))))

(fn `UserConstructionScript`)