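; OrbitPawn is a camera pawn that continuously orbits around its own origin on a spring arm.
; Each tick it adds yaw input at an adjustable speed and copies the control rotation to the spring arm's relative rotation.
; Hard-coded keys change the orbit speed, raise, lower or rotate the camera, and quit the game.
; The mouse wheel zooms by changing arm length, with no limits applied.
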(event `self.ReceiveBeginPlay`)

(event `self.ReceiveTick`
  (params (DeltaSeconds :type "Float (single-precision)"))
  (`self.AddControllerYawInput` (`self.YawRotSpeed`))
  (`SceneComponent.K2_SetRelativeRotation` (`self.SpringArm`) (`self.GetControlRotation`) false false))

(event `Key|MouseScrollUp`
  (params (Key :type "Key Structure"))
  (bind _springarm (`self.SpringArm`))
  (:`Pressed`
    (set `SpringArmComponent.TargetArmLength` (- (`SpringArmComponent.TargetArmLength` _springarm) 10.0) _springarm)))

(event `Key|MouseScrollDown`
  (params (Key :type "Key Structure"))
  (bind _springarm (`self.SpringArm`))
  (:`Pressed`
    (set `SpringArmComponent.TargetArmLength` (+ (`SpringArmComponent.TargetArmLength` _springarm) 10.0) _springarm)))

(event `Key|E`
  (params (Key :type "Key Structure"))
  (:`Pressed`
    (`SceneComponent.K2_AddWorldOffset` (`self.Camera`) (0.0 0.0 10.0) false false)))

(event `Key|Q`
  (params (Key :type "Key Structure"))
  (:`Pressed`
    (`SceneComponent.K2_AddWorldOffset` (`self.Camera`) (0.0 0.0 -10.0) false false)))

(event `Key|R`
  (params (Key :type "Key Structure"))
  (:`Pressed`
    (`SceneComponent.K2_AddRelativeRotation` (`self.Camera`) (struct :`Pitch` 0.5) false false)))

(event `Key|T`
  (params (Key :type "Key Structure"))
  (:`Pressed`
    (`SceneComponent.K2_AddRelativeRotation` (`self.Camera`) (struct :`Pitch` -0.5) false false)))

(event `Key|A`
  (params (Key :type "Key Structure"))
  (:`Pressed`
    (set `self.YawRotSpeed` (+ (`self.YawRotSpeed`) 0.002))))

(event `Key|S`
  (params (Key :type "Key Structure"))
  (:`Pressed`
    (set `self.YawRotSpeed` (+ (`self.YawRotSpeed`) -0.002))))

(event `Key|Escape`
  (params (Key :type "Key Structure"))
  (:`Pressed`
    (`KismetSystemLibrary.QuitGame` null "Quit")))

(fn `UserConstructionScript`)