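; Voxel video actor that plays video through a voxel render component.
; The construction script assigns the VoxelVideoSource component as the source of VoxelRender.
; Play, Pause and Stop forward directly to that source, while TogglePlay switches between play and pause using an IsPlaying flag.
; Only TogglePlay updates that flag, so direct Play, Pause or Stop calls leave it unchanged.
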(fn `Pause`
  (`VoxelVideoSourceComponent.Pause` (`self.VoxelVideoSource`)))

(fn `Play`
  (`VoxelVideoSourceComponent.Play` (`self.VoxelVideoSource`)))

(fn `Stop`
  (`VoxelVideoSourceComponent.Stop` (`self.VoxelVideoSource`)))

(fn `TogglePlay`
  (bind _voxelvideosource (`self.VoxelVideoSource`))
  (if (`self.IsPlaying`)
    (`VoxelVideoSourceComponent.Pause` _voxelvideosource)
    (set `self.IsPlaying` false)
    (else
      (`VoxelVideoSourceComponent.Play` _voxelvideosource)
      (set `self.IsPlaying` true))))

(fn `UserConstructionScript`
  (set `VoxelRenderComponent.VoxelSource` (`self.VoxelVideoSource`) (`self.VoxelRender`)))