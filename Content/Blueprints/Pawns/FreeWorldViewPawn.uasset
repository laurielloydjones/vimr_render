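; Free-fly world view pawn that lets the player adjust movement speed and camera zoom at runtime.
; Mouse wheel input scales the FloatingPawnMovement max speed by a multiplier, clamped between configurable walk speed bounds.
; ZoomIn and ZoomOut actions step the player camera manager's default FOV within fixed limits.
; Middle mouse restores the FOV captured at BeginPlay, which also sets the starting speed.
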(event `self.ReceiveBeginPlay`
  (set `self.DefaultCameraFOV` (`PlayerCameraManager.GetFOVAngle` (`GameplayStatics.GetPlayerCameraManager` 0)))
  (bind _asfloating_pawn_movement (cast `FloatingPawnMovement` (`self.MovementComponent`)))
  (set `FloatingPawnMovement.MaxSpeed` 600.0 _asfloating_pawn_movement))

(event `Key|MouseScrollUp`
  (params (Key :type "Key Structure"))
  ;[1 1 1] Movement Speed Control
  (:`Pressed`
    (bind _asfloating_pawn_movement (cast `FloatingPawnMovement` (`self.MovementComponent`) :!label _label))
    (bind _validatedwalkspeed (`self.CheckWalkSpeedBounds` (+ (`MovementComponent.GetMaxSpeed` _asfloating_pawn_movement) (* (`self.GetInputAxisKeyValue`) (`self.MovementSpeedMultiplier`)))))
    (bind _asfloating_pawn_movement_2 (cast `FloatingPawnMovement` (`self.MovementComponent`)))
    (set `FloatingPawnMovement.MaxSpeed` _validatedwalkspeed _asfloating_pawn_movement_2)))

(event `Key|MouseScrollDown`
  (params (Key :type "Key Structure"))
  ;[1 1 1] Movement Speed Control
  (:`Pressed`
    (goto _label)))

(event `InputAction|ZoomIn`
  (params (Key :type "Key Structure"))
  (bind _returnvalue (`GameplayStatics.GetPlayerCameraManager` 0))
  ;[1 1 1] Zoom Functions
  (:`Pressed`
    (bind _validatedfov (`self.CheckFOVBounds` (- (`PlayerCameraManager.GetFOVAngle` _returnvalue) (`self.StepSize`))))
    (set `PlayerCameraManager.DefaultFOV` _validatedfov _returnvalue)))

(event `InputAction|ZoomOut`
  (params (Key :type "Key Structure"))
  (bind _returnvalue (`GameplayStatics.GetPlayerCameraManager` 0))
  ;[1 1 1] Zoom Functions
  (:`Pressed`
    (bind _validatedfov (`self.CheckFOVBounds` (+ (`PlayerCameraManager.GetFOVAngle` _returnvalue) (`self.StepSize`))))
    (set `PlayerCameraManager.DefaultFOV` _validatedfov _returnvalue)))

(event `Key|MiddleMouseButton`
  (params (Key :type "Key Structure"))
  ;[1 1 1] Zoom Functions
  (:`Pressed`
    (set `PlayerCameraManager.DefaultFOV` (`self.DefaultCameraFOV`) (`GameplayStatics.GetPlayerCameraManager` 0))))

(fn `CheckFOVBounds`
  (params (CurrentFOV :type "Float (double-precision)"))
  (returns (ValidatedFOV :type "Float (double-precision)"))
  (locals (TmpFOV :type "Float (double-precision)"))
  (bind _output_get (set `local.TmpFOV` CurrentFOV))
  (if (> _output_get 135.0)
    (set `local.TmpFOV` 135.0)
    (elif (<= _output_get 15.0)
      (set `local.TmpFOV` 15.0)))
  (return (`local.TmpFOV`)))

(fn `CheckWalkSpeedBounds`
  (params (CurrentWalkSpeed :type "Float (double-precision)"))
  (returns (ValidatedWalkSpeed :type "Float (double-precision)"))
  (locals (TempWalkSpeed :type "Float (double-precision)"))
  (bind _minwalkspeed (`self.MinWalkSpeed`))
  (bind _maxwalkspeed (`self.MaxWalkSpeed`))
  (bind _output_get (set `local.TempWalkSpeed` CurrentWalkSpeed))
  (if (>= _output_get _maxwalkspeed)
    (set `local.TempWalkSpeed` _maxwalkspeed)
    (elif (<= (`local.TempWalkSpeed`) _minwalkspeed)
      (set `local.TempWalkSpeed` _minwalkspeed)))
  (return (`local.TempWalkSpeed`)))

(fn `UserConstructionScript`)